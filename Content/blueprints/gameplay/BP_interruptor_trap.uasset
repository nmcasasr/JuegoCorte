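; Trap switch that punishes the player for pressing the action input while standing in its Box volume.
; The Box overlap enables input on the actor when the master_player enters and disables it when they leave.
; Each action press plays an error sound and subtracts a fixed amount from the Life of the player cast on overlap.
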(event OnComponentBeginOverlap(Box)
  (params (OverlappedComponent :type Primitive%20Component%20Object%20Reference) (OtherActor :type Actor%20Object%20Reference) (OtherComp :type Primitive%20Component%20Object%20Reference) (OtherBodyIndex :type Integer) (bFromSweep :type Boolean) (SweepResult :type Hit%20Result%20Structure%20%28by%20ref%29))
  (bind _asmaster_player (Utilities|Casting|CastTomaster_player OtherActor))
  (Input|EnableInput (Game|GetPlayerController 0)))

(event OnComponentEndOverlap(Box)
  (params (OverlappedComponent :type Primitive%20Component%20Object%20Reference) (OtherActor :type Actor%20Object%20Reference) (OtherComp :type Primitive%20Component%20Object%20Reference) (OtherBodyIndex :type Integer))
  (Utilities|Casting|CastTomaster_player OtherActor)
  (Input|DisableInput (Game|GetPlayerController 0)))

(event Input|ActionEvents|InputActionaction
  (params (Key :type Key%20Structure))
  (:Pressed
    (Audio|PlaySound2D "/Game/Sounds/142608__autistic-lucario__error.142608__autistic-lucario__error" 1.0 1.0 0.0 0 0)
    (Variables|/Game/blueprints/player/master_player.master_player_C|Setlife (stale OnComponentBeginOverlap(Box) _asmaster_player) (- (Variables|/Game/blueprints/player/master_player.master_player_C|Getlife (stale OnComponentBeginOverlap(Box) _asmaster_player)) 0.5))))

(fn ConstructionScript)