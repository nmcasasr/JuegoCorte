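; BP_door_start is a door that opens when a player with enough keys enters its trigger box.
; On overlap it casts to master_player and compares NumberKeys against TipeDoor, then plays a shutter sound and a timeline that moves the SMDoor mesh's relative location.
; Leaving the box plays the same sound and reverses the timeline, without repeating the key check.
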(event OnComponentBeginOverlap(Box)
  (params (OverlappedComponent :type Primitive%20Component%20Object%20Reference) (OtherActor :type Actor%20Object%20Reference) (OtherComp :type Primitive%20Component%20Object%20Reference) (OtherBodyIndex :type Integer) (bFromSweep :type Boolean) (SweepResult :type Hit%20Result%20Structure%20%28by%20ref%29))
  (bind _asmaster_player (Utilities|Casting|CastTomaster_player OtherActor))
  (if (>= (Variables|/Game/blueprints/player/master_player.master_player_C|GetnumberKeys _asmaster_player) (Variables|Default|GetTipe%20Door))
    (Audio|PlaySound2D "/Game/Sounds/transition_shutter_002.transition_shutter_002" 1.0 1.0 0.0 0 0)
    (bind _newtrack_0 (Timeline|Timeline_0 Play)
      (:Update
        (Transformation|SetRelativeLocation (Variables|Default|GetSM_door) _newtrack_0 false false)))))

(event OnComponentEndOverlap(Box)
  (params (OverlappedComponent :type Primitive%20Component%20Object%20Reference) (OtherActor :type Actor%20Object%20Reference) (OtherComp :type Primitive%20Component%20Object%20Reference) (OtherBodyIndex :type Integer))
  (Utilities|Casting|CastTomaster_player OtherActor)
  (Audio|PlaySound2D "/Game/Sounds/transition_shutter_002.transition_shutter_002" 1.0 1.0 0.0 0 0)
  (bind _newtrack_0 (Timeline|Timeline_0 Reverse)
    (:Update
      (Transformation|SetRelativeLocation (Variables|Default|GetSM_door) _newtrack_0 false false))))

(fn ConstructionScript)