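; Interruptor master Blueprint: a switch the player presses to activate a linked DoorButton.
; A Box overlap with the master_player enables input on the actor, and leaving it disables input.
; Pressing the action input sets DoorButton.Pressed, plays a beep, and turns its own light and both DoorButton lights green.
; The press is one-way, with no reset in this graph.
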(event OnComponentBeginOverlap(Box)
  (params (OverlappedComponent :type Primitive%20Component%20Object%20Reference) (OtherActor :type Actor%20Object%20Reference) (OtherComp :type Primitive%20Component%20Object%20Reference) (OtherBodyIndex :type Integer) (bFromSweep :type Boolean) (SweepResult :type Hit%20Result%20Structure%20%28by%20ref%29))
  (Utilities|Casting|CastTomaster_player OtherActor)
  (Input|EnableInput (Game|GetPlayerController 0)))

(event OnComponentEndOverlap(Box)
  (params (OverlappedComponent :type Primitive%20Component%20Object%20Reference) (OtherActor :type Actor%20Object%20Reference) (OtherComp :type Primitive%20Component%20Object%20Reference) (OtherBodyIndex :type Integer))
  (Utilities|Casting|CastTomaster_player OtherActor)
  (Input|DisableInput (Game|GetPlayerController 0)))

(event Input|ActionEvents|InputActionaction
  (params (Key :type Key%20Structure))
  (bind _door_button (Variables|Default|Getdoor_button))
  (:Pressed
    (Variables|/Game/blueprints/gameplay/BP_door_button.BP_door_button_C|Setpressed _door_button true)
    (Audio|PlaySound2D "/Game/Sounds/220206__gameaudio__beep-space-button.220206__gameaudio__beep-space-button" 1.0 1.0 0.0 0 0)
    (Rendering|Components|Light|SetLightColor (Variables|Default|GetPointLight) "(R=0.049789,G=1.000000,B=0.000000,A=1.000000)" true)
    (Rendering|Components|Light|SetLightColor (Variables|/Game/blueprints/gameplay/BP_door_button.BP_door_button_C|GetPointLight1 _door_button) "(R=0.089306,G=1.000000,B=0.000000,A=1.000000)" true)))

(fn ConstructionScript)