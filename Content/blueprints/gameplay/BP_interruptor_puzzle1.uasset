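; Four-switch light puzzle that disarms a linked LaserDoor when all four lights are green.
; Overlap boxes enable input for the player and record which switch is in range.
; Pressing action flips that switch's fixed subset of boolean states, recoloring the point lights red or green.
; Every press then checks for all true, which clears the door's damage flag, swaps its laser materials and turns its lights green, with no re-arm.
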(event OnComponentBeginOverlap(Box3)
  (params (OverlappedComponent :type Primitive%20Component%20Object%20Reference) (OtherActor :type Actor%20Object%20Reference) (OtherComp :type Primitive%20Component%20Object%20Reference) (OtherBodyIndex :type Integer) (bFromSweep :type Boolean) (SweepResult :type Hit%20Result%20Structure%20%28by%20ref%29))
  (Utilities|Casting|CastTomaster_player OtherActor)
  (Input|EnableInput (Game|GetPlayerController 0))
  (Variables|Default|SetnumberButton 3))

(event OnComponentBeginOverlap(Box2)
  (params (OverlappedComponent :type Primitive%20Component%20Object%20Reference) (OtherActor :type Actor%20Object%20Reference) (OtherComp :type Primitive%20Component%20Object%20Reference) (OtherBodyIndex :type Integer) (bFromSweep :type Boolean) (SweepResult :type Hit%20Result%20Structure%20%28by%20ref%29))
  (Utilities|Casting|CastTomaster_player OtherActor)
  (Input|EnableInput (Game|GetPlayerController 0))
  (Variables|Default|SetnumberButton 2))

(event OnComponentBeginOverlap(Box1)
  (params (OverlappedComponent :type Primitive%20Component%20Object%20Reference) (OtherActor :type Actor%20Object%20Reference) (OtherComp :type Primitive%20Component%20Object%20Reference) (OtherBodyIndex :type Integer) (bFromSweep :type Boolean) (SweepResult :type Hit%20Result%20Structure%20%28by%20ref%29))
  (Utilities|Casting|CastTomaster_player OtherActor)
  (Input|EnableInput (Game|GetPlayerController 0))
  (Variables|Default|SetnumberButton 1))

(event OnComponentEndOverlap(Box1)
  (params (OverlappedComponent :type Primitive%20Component%20Object%20Reference) (OtherActor :type Actor%20Object%20Reference) (OtherComp :type Primitive%20Component%20Object%20Reference) (OtherBodyIndex :type Integer))
  (Utilities|Casting|CastTomaster_player OtherActor)
  (Input|DisableInput (Game|GetPlayerController 0)))

(event OnComponentEndOverlap(Box2)
  (params (OverlappedComponent :type Primitive%20Component%20Object%20Reference) (OtherActor :type Actor%20Object%20Reference) (OtherComp :type Primitive%20Component%20Object%20Reference) (OtherBodyIndex :type Integer))
  (Utilities|Casting|CastTomaster_player OtherActor)
  (Input|DisableInput (Game|GetPlayerController 0)))

(event OnComponentEndOverlap(Box3)
  (params (OverlappedComponent :type Primitive%20Component%20Object%20Reference) (OtherActor :type Actor%20Object%20Reference) (OtherComp :type Primitive%20Component%20Object%20Reference) (OtherBodyIndex :type Integer))
  (Utilities|Casting|CastTomaster_player OtherActor)
  (Input|DisableInput (Game|GetPlayerController 0)))

(event OnComponentBeginOverlap(Box31)
  (params (OverlappedComponent :type Primitive%20Component%20Object%20Reference) (OtherActor :type Actor%20Object%20Reference) (OtherComp :type Primitive%20Component%20Object%20Reference) (OtherBodyIndex :type Integer) (bFromSweep :type Boolean) (SweepResult :type Hit%20Result%20Structure%20%28by%20ref%29))
  (Utilities|Casting|CastTomaster_player OtherActor)
  (Input|EnableInput (Game|GetPlayerController 0))
  (Variables|Default|SetnumberButton 4))

(event OnComponentEndOverlap(Box31)
  (params (OverlappedComponent :type Primitive%20Component%20Object%20Reference) (OtherActor :type Actor%20Object%20Reference) (OtherComp :type Primitive%20Component%20Object%20Reference) (OtherBodyIndex :type Integer))
  (Utilities|Casting|CastTomaster_player OtherActor)
  (Input|DisableInput (Game|GetPlayerController 0)))

(event Input|ActionEvents|InputActionaction
  (params (Key :type Key%20Structure))
  (bind _laserdoor (Variables|Default|GetlaserDoor))
  (:Pressed
    (switch int (Variables|Default|GetnumberButton)
      (:1
        (if (Variables|Default|Getbool1)
          (Variables|Default|Setbool1 false)
          (Rendering|Components|Light|SetLightColor (Variables|Default|GetPointLight1) "(R=1.000000,G=0.000000,B=0.000000,A=1.000000)" true)
          (else
            (Variables|Default|Setbool1 true)
            (Rendering|Components|Light|SetLightColor (Variables|Default|GetPointLight1) "(R=0.089306,G=1.000000,B=0.000000,A=1.000000)" true)))
        (if (Variables|Default|Getbool2)
          (Variables|Default|Setbool2 true)
          (Rendering|Components|Light|SetLightColor (Variables|Default|GetPointLight2) "(R=0.031630,G=1.000000,B=0.000000,A=1.000000)" true)
          (else
            (Variables|Default|Setbool2 false)
            (Rendering|Components|Light|SetLightColor (Variables|Default|GetPointLight2) "(R=1.000000,G=0.000000,B=0.000000,A=1.000000)" true)))
        (if (Variables|Default|Getbool3)
          (Variables|Default|Setbool3 false)
          (Rendering|Components|Light|SetLightColor (Variables|Default|GetPointLight3) "(R=1.000000,G=0.000000,B=0.000000,A=1.000000)" true)
          (else
            (Variables|Default|Setbool3 true)
            (Rendering|Components|Light|SetLightColor (Variables|Default|GetPointLight3) "(R=0.031630,G=1.000000,B=0.000000,A=1.000000)" true)))
        (if (Variables|Default|Getbool4)
          (Variables|Default|Setbool4 true)
          (Rendering|Components|Light|SetLightColor (Variables|Default|GetPointLight31) "(R=0.089306,G=1.000000,B=0.000000,A=1.000000)" true)
          (else
            (Variables|Default|Setbool4 false)
            (Rendering|Components|Light|SetLightColor (Variables|Default|GetPointLight31) "(R=1.000000,G=0.000000,B=0.000000,A=1.000000)" true))))
      (:2
        (if (Variables|Default|Getbool1)
          (Variables|Default|Setbool1 true)
          (Rendering|Components|Light|SetLightColor (Variables|Default|GetPointLight1) "(R=0.031630,G=1.000000,B=0.000000,A=1.000000)" true)
          (else
            (Variables|Default|Setbool1 false)
            (Rendering|Components|Light|SetLightColor (Variables|Default|GetPointLight1) "(R=1.000000,G=0.000000,B=0.000000,A=1.000000)" true)))
        (if (Variables|Default|Getbool2)
          (Variables|Default|Setbool2 false)
          (Rendering|Components|Light|SetLightColor (Variables|Default|GetPointLight2) "(R=1.000000,G=0.000000,B=0.000000,A=1.000000)" true)
          (else
            (Variables|Default|Setbool2 true)
            (Rendering|Components|Light|SetLightColor (Variables|Default|GetPointLight2) "(R=0.089306,G=1.000000,B=0.000000,A=1.000000)" true)))
        (if (Variables|Default|Getbool3)
          (Variables|Default|Setbool3 false)
          (Rendering|Components|Light|SetLightColor (Variables|Default|GetPointLight3) "(R=1.000000,G=0.000000,B=0.000000,A=1.000000)" true)
          (else
            (Variables|Default|Setbool3 true)
            (Rendering|Components|Light|SetLightColor (Variables|Default|GetPointLight3) "(R=0.089306,G=1.000000,B=0.000000,A=1.000000)" true)))
        (if (Variables|Default|Getbool4)
          (Variables|Default|Setbool4 true)
          (Rendering|Components|Light|SetLightColor (Variables|Default|GetPointLight31) "(R=0.089306,G=1.000000,B=0.000000,A=1.000000)" true)
          (else
            (Variables|Default|Setbool4 false)
            (Rendering|Components|Light|SetLightColor (Variables|Default|GetPointLight31) "(R=1.000000,G=0.000000,B=0.000000,A=1.000000)" true))))
      (:3
        (if (Variables|Default|Getbool1)
          (Variables|Default|Setbool1 true)
          (Rendering|Components|Light|SetLightColor (Variables|Default|GetPointLight1) "(R=0.089306,G=1.000000,B=0.000000,A=1.000000)" true)
          (else
            (Variables|Default|Setbool1 false)
            (Rendering|Components|Light|SetLightColor (Variables|Default|GetPointLight1) "(R=1.000000,G=0.000000,B=0.000000,A=1.000000)" true)))
        (if (Variables|Default|Getbool2)
          (Variables|Default|Setbool2 false)
          (Rendering|Components|Light|SetLightColor (Variables|Default|GetPointLight2) "(R=1.000000,G=0.000000,B=0.000000,A=1.000000)" true)
          (else
            (Variables|Default|Setbool2 true)
            (Rendering|Components|Light|SetLightColor (Variables|Default|GetPointLight2) "(R=0.089306,G=1.000000,B=0.000000,A=1.000000)" true)))
        (if (Variables|Default|Getbool3)
          (Variables|Default|Setbool3 false)
          (Rendering|Components|Light|SetLightColor (Variables|Default|GetPointLight3) "(R=1.000000,G=0.000000,B=0.000000,A=1.000000)" true)
          (else
            (Variables|Default|Setbool3 true)
            (Rendering|Components|Light|SetLightColor (Variables|Default|GetPointLight3) "(R=0.089306,G=1.000000,B=0.000000,A=1.000000)" true)))
        (if (Variables|Default|Getbool4)
          (Variables|Default|Setbool4 false)
          (Rendering|Components|Light|SetLightColor (Variables|Default|GetPointLight31) "(R=1.000000,G=0.000000,B=0.000000,A=1.000000)" true)
          (else
            (Variables|Default|Setbool4 true)
            (Rendering|Components|Light|SetLightColor (Variables|Default|GetPointLight31) "(R=0.089306,G=1.000000,B=0.000000,A=1.000000)" true))))
      (:4
        (if (Variables|Default|Getbool1)
          (Variables|Default|Setbool1 true)
          (Rendering|Components|Light|SetLightColor (Variables|Default|GetPointLight1) "(R=0.089306,G=1.000000,B=0.000000,A=1.000000)" true)
          (else
            (Variables|Default|Setbool1 false)
            (Rendering|Components|Light|SetLightColor (Variables|Default|GetPointLight1) "(R=1.000000,G=0.000000,B=0.000000,A=1.000000)" true)))
        (if (Variables|Default|Getbool2)
          (Variables|Default|Setbool2 true)
          (Rendering|Components|Light|SetLightColor (Variables|Default|GetPointLight2) "(R=0.089306,G=1.000000,B=0.000000,A=1.000000)" true)
          (else
            (Variables|Default|Setbool2 false)
            (Rendering|Components|Light|SetLightColor (Variables|Default|GetPointLight2) "(R=1.000000,G=0.000000,B=0.000000,A=1.000000)" true)))
        (if (Variables|Default|Getbool3)
          (Variables|Default|Setbool3 false)
          (Rendering|Components|Light|SetLightColor (Variables|Default|GetPointLight3) "(R=1.000000,G=0.000000,B=0.000000,A=1.000000)" true)
          (else
            (Variables|Default|Setbool3 true)
            (Rendering|Components|Light|SetLightColor (Variables|Default|GetPointLight3) "(R=0.089306,G=1.000000,B=0.000000,A=1.000000)" true)))
        (if (Variables|Default|Getbool4)
          (Variables|Default|Setbool4 false)
          (Rendering|Components|Light|SetLightColor (Variables|Default|GetPointLight31) "(R=1.000000,G=0.000000,B=0.000000,A=1.000000)" true)
          (else
            (Variables|Default|Setbool4 true)
            (Rendering|Components|Light|SetLightColor (Variables|Default|GetPointLight31) "(R=0.089306,G=1.000000,B=0.000000,A=1.000000)" true)))))
    (if (Math|Boolean|ANDBoolean (Variables|Default|Getbool1) (Variables|Default|Getbool2) (Variables|Default|Getbool3) (Variables|Default|Getbool4))
      (Variables|/Game/blueprints/gameplay/BP_door_laser.BP_door_laser_C|SetboolDaño _laserdoor false)
      (Rendering|Material|SetMaterial (Variables|/Game/blueprints/gameplay/BP_door_laser.BP_door_laser_C|Get%20Cube3 _laserdoor) 0 "/Game/GT_SELECT18/laser_Inst.laser_Inst")
      (Rendering|Material|SetMaterial (Variables|/Game/blueprints/gameplay/BP_door_laser.BP_door_laser_C|Get%20Cube2 _laserdoor) 0 "/Game/GT_SELECT18/laser_Inst.laser_Inst")
      (Rendering|Material|SetMaterial (Variables|/Game/blueprints/gameplay/BP_door_laser.BP_door_laser_C|GetCube _laserdoor) 0 "/Game/GT_SELECT18/laser_Inst.laser_Inst")
      (Rendering|Components|Light|SetLightColor (Variables|/Game/blueprints/gameplay/BP_door_laser.BP_door_laser_C|GetRectLight _laserdoor) "(R=0.031630,G=1.000000,B=0.000000,A=1.000000)" true)
      (Rendering|Components|Light|SetLightColor (Variables|/Game/blueprints/gameplay/BP_door_laser.BP_door_laser_C|GetRectLight1 _laserdoor) "(R=0.031630,G=1.000000,B=0.000000,A=1.000000)" true)
      (Rendering|Components|Light|SetLightColor (Variables|/Game/blueprints/gameplay/BP_door_laser.BP_door_laser_C|GetRectLight11 _laserdoor) "(R=0.031630,G=1.000000,B=0.000000,A=1.000000)" true))))

(fn ConstructionScript)