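; BP_item_master is an item Blueprint that animates its Cubo component's relative location from the start of play.
; On BeginPlay, a switch on Tipo selects one of three timelines.
; The chosen timeline's track output sets the component's relative location on each update, with sweep and teleport off.
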(event EventBeginPlay
  (switch int (Variables|Default|Gettipo)
    (:0
      (bind _newtrack_1 (Timeline|Timeline_1 Play)
        (:Update
          (Transformation|SetRelativeLocation (Variables|Default|Getcubo) _newtrack_1 false false))))
    (:1
      (bind _newtrack_1_2 (Timeline|Timeline_2 Play)
        (:Update
          (Transformation|SetRelativeLocation (Variables|Default|Getcubo) _newtrack_1_2 false false))))
    (:2
      (bind _newtrack_1_3 (Timeline|Timeline_3 Play)
        (:Update
          (Transformation|SetRelativeLocation (Variables|Default|Getcubo) _newtrack_1_3 false false))))))

(fn ConstructionScript)