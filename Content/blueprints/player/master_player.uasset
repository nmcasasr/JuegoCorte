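; Player character Blueprint that creates the general HUD widget on BeginPlay and handles jumping, running and axis-driven camera look.
; Movement input follows the controller's yaw and roll with pitch zeroed, while the run action switches max walk speed between walking and running values.
; Tick converts the key count to a string, caps Life at full, and destroys the actor and reopens level1 when Life is nearly depleted.
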(event EventBeginPlay
  (bind _returnvalue (UserInterface|CreateWidget "/Game/blueprints/WBP_general.WBP_general_C"))
  (UserInterface|Viewport|AddtoViewport _returnvalue 0))

(event EventTick
  (params (DeltaSeconds :type Float%20%28single-precision%29))
  (Variables|Default|SetkeyString (Utilities|String|ToString(Integer) (Variables|Default|GetnumberKeys)))
  (if (<= (Variables|Default|Getlife) 0.01)
    (Actor|DestroyActor)
    (Game|OpenLevel(byName) "level1")
    (elif (> (Variables|Default|Getlife) 1.0)
      (Variables|Default|Setlife 1.0))))

(event Input|ActionEvents|InputActionjump
  (params (Key :type Key%20Structure))
  (:Pressed
    (Character|Jump)))

(event Input|ActionEvents|InputActionrun
  (params (Key :type Key%20Structure))
  (bind _charactermovement (Variables|Character|GetCharacterMovement))
  (:Pressed
    (Variables|/Script/Engine.CharacterMovementComponent|SetMaxWalkSpeed _charactermovement 6e+02))
  (:Released
    (Variables|/Script/Engine.CharacterMovementComponent|SetMaxWalkSpeed _charactermovement 2.5e+02)))

(event Input|ActionEvents|InputActionaction
  (params (Key :type Key%20Structure)))

(event Input|ActionEvents|InputActionreset
  (params (Key :type Key%20Structure)))

(event Input|AxisEvents|InputAxisright/left
  (params (AxisValue :type Float%20%28single-precision%29))
  (bind _returnvalue (Game|GetPlayerController 0))
  (bind _returnvalue_2 (Pawn|GetControlRotation _returnvalue :!class /Script/Engine.Controller))
  (Pawn|Input|AddMovementInput (Math|Vector|GetRightVector (Math|Rotator|MakeRotator (.roll _returnvalue_2) 0.0 (.yaw _returnvalue_2))) AxisValue false))

(event Input|AxisEvents|InputAxisfront/back
  (params (AxisValue :type Float%20%28single-precision%29))
  (bind _returnvalue (Game|GetPlayerController 0))
  (bind _returnvalue_2 (Pawn|GetControlRotation _returnvalue :!class /Script/Engine.Controller))
  (Pawn|Input|AddMovementInput (Math|Vector|GetForwardVector (Math|Rotator|MakeRotator (.roll _returnvalue_2) 0.0 (.yaw _returnvalue_2))) AxisValue false))

(event Input|AxisEvents|InputAxislookSides
  (params (AxisValue :type Float%20%28single-precision%29))
  (Pawn|Input|AddControllerYawInput AxisValue))

(event Input|AxisEvents|InputAxislookUpDown
  (params (AxisValue :type Float%20%28single-precision%29))
  (Pawn|Input|AddControllerPitchInput AxisValue))

(fn ConstructionScript)